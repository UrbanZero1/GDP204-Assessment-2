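; Dialogue manager actor that runs a visual-novel story about Jordan, from main menu to an affection-based ending.
; It builds scenarios from DataTables, then steps through lines, swapping background, character and dialogue widgets.
; Choices adjust JordanAffection, which picks conditional lines and the ending.
; It also handles menu/gameplay music, save/load to one slot, and gamepad stick cursor control.
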(event Custom|DisplayCurrentDialogue
  (Variables|Default|SetbDisplaying true)
  (if (Variables|Default|GetbScenarioChange)
    (bind _backgroundtexture (CallFunction|GetScenarioBackground (Variables|Default|GetCurrentScenario)))
    (Default|ChangeBackground (Variables|Default|GetBackgroundWidget) _backgroundtexture)
    (Default|ResetCharacter (Variables|Default|GetCharacterDisplayWidget))
    (Variables|Default|SetbScenarioChange false))
  (bind _output_get (Variables|Default|SetCurrentDialogue (Utilities|Array|Get(acopy) (.dialoguearray (Variables|Default|GetCurrentScenario)) (Variables|Default|GetCurrentDialogueIndex))))
  (CallFunction|DisplayCharacter (.speakername _output_get) (.characteremotion _output_get))
  (if (.bcondition _output_get)
    (if (> (Variables|Default|GetJordanAffection) 1)
      (Variables|Default|SetDialogueText (Utilities|Array|Get(acopy) (.dialogues _output_get) 1))
      (else
        (Variables|Default|SetDialogueText (Utilities|Array|Get(acopy) (.dialogues _output_get)) :!label _label)))
    (else
      (goto _label)))
  (Widget|RemovefromParent (Variables|Default|GetCurrentDialogueWidget))
  (bind _returnvalue (UserInterface|CreateWidget "/Game/DialogueSystem/Widgets/WI_Dialogue.WI_Dialogue_C" (Game|GetPlayerController 0) (.speakername _output_get) (Variables|Default|GetDialogueText) self))
  (bind _output_get_2 (Variables|Default|SetCurrentDialogueWidget _returnvalue))
  (UserInterface|Viewport|AddtoViewport _output_get_2 2)
  (if (.bhasresponse (Variables|Default|GetCurrentDialogue))
    (Variables|Default|SetbResolveChoices true)
    (else
      (Utilities|ResolveDialogue))))

(event Custom|FinishedDisplaying
  (Variables|Default|SetbDisplaying false))

(event Custom|StartGame
  (CallFunction|PlayGameMusic)
  (bind _output_get (Utilities|GameInit))
  (bind _output_get_2 (Variables|Default|SetCurrentScenario (Utilities|Array|Get(acopy) _output_get (Variables|Default|GetCurrentScenarioIndex))))
  (bind _backgroundtexture (CallFunction|GetScenarioBackground _output_get_2))
  (Default|ChangeBackground (Variables|Default|GetBackgroundWidget) _backgroundtexture)
  (bind _returnvalue (UserInterface|CreateWidget "/Game/DialogueSystem/Widgets/WI_Dialogue.WI_Dialogue_C" 0 "Init" "" 0))
  (Variables|Default|SetCurrentDialogueWidget _returnvalue)
  (CallFunction|DisplayCurrentDialogue))

(event Custom|JordanEnding
  (Variables|Default|SetbDisplaying true)
  (Widget|RemovefromParent (Variables|Default|GetBackgroundWidget))
  (Widget|RemovefromParent (Variables|Default|GetInGameOptionsWidget))
  (Widget|RemovefromParent (Variables|Default|GetCurrentDialogueWidget))
  (if (> (Variables|Default|GetJordanAffection) 0)
    (Default|ChangeCharacter (Variables|Default|GetCharacterDisplayWidget) "/Game/Assets/Guy_1/Happy.Happy")
    (bind _returnvalue (UserInterface|CreateWidget "/Game/DialogueSystem/Widgets/WI_Dialogue.WI_Dialogue_C" 0 "Internal" "Nearly everyday I see Jordan at our regular café meetups. We have a quiet but sustainable friendship. We even planned a museum day for the future. It seems like I made a long-lasting friend. " self))
    (UserInterface|Viewport|AddtoViewport _returnvalue 0)
    (Utilities|FlowControl|Delay 1e+01)
    (Game|QuitGame 0 "Quit" false)
    (else
      (Default|ChangeCharacter (Variables|Default|GetCharacterDisplayWidget) "/Game/Assets/Guy_1/Normal.Normal")
      (bind _returnvalue_2 (UserInterface|CreateWidget "/Game/DialogueSystem/Widgets/WI_Dialogue.WI_Dialogue_C" 0 "Internal" "It’s post-graduation. Jordans face shows up in my memories every now and then, but we both must live our separate lives. It was nice while it lasted. " self))
      (UserInterface|Viewport|AddtoViewport _returnvalue_2 0)
      (Utilities|FlowControl|Delay 1e+01)
      (Game|QuitGame 0 "Quit" false))))

(event EventBeginPlay
  (bind _returnvalue (Game|GetPlayerController 0))
  (Variables|/Script/Engine.PlayerController|SetbShowMouseCursor _returnvalue true)
  (Input|EnableInput _returnvalue)
  (bind _returnvalue_2 (UserInterface|CreateWidget "/Game/DialogueSystem/Widgets/WI_MainMenu.WI_MainMenu_C" 0 self))
  (bind _output_get (Variables|Default|SetMainMenuWidget _returnvalue_2))
  (UserInterface|Viewport|AddtoViewport _output_get 0)
  (bind _returnvalue_3 (Audio|CreateSound2D "/Game/Assets/Audio/Music/GameplayCue.GameplayCue" 1.0 1.0 0.0 0))
  (Variables|Default|SetGameplayMusic _returnvalue_3)
  (bind _returnvalue_4 (Audio|CreateSound2D "/Game/Assets/Audio/Music/MainMenuCue.MainMenuCue" 1.0 1.0 0.0 0))
  (bind _output_get_2 (Variables|Default|SetMainMenuMusic _returnvalue_4))
  (Audio|Components|Audio|Play _output_get_2 0.0))

(event Input|ActionEvents|InputActionClick
  (params (Key :type Key%20Structure :default "None"))
  (:Pressed
    (if (not (Variables|Default|GetbDisplaying))
      (if (Variables|Default|GetbEnding)
        (CallFunction|JordanEnding)
        (elif (Variables|Default|GetbResolveChoices)
          (Variables|Default|SetbDisplaying true)
          (Widget|RemovefromParent (Variables|Default|GetCurrentDialogueWidget))
          (bind _returnvalue (UserInterface|CreateWidget "/Game/DialogueSystem/Widgets/WI_ChoiceSelection.WI_ChoiceSelection_C" (Game|GetPlayerController 0) self (.responses (Variables|Default|GetCurrentDialogue))))
          (bind _output_get (Variables|Default|SetChoicesWidget _returnvalue))
          (UserInterface|Viewport|AddtoViewport _output_get 0)
          (else
            (CallFunction|DisplayCurrentDialogue)))))))

(event Input|ActionEvents|InputActionDialogueNext
  (params (Key :type Key%20Structure :default "None"))
  (:Pressed
    (Class|WidgetInteractionComponent|PressKey (Variables|Default|GetWidgetInteraction) "LeftMouseButton" false)))

(event Input|ActionEvents|InputActionDialogueNext
  (params (Key :type Key%20Structure :default "None"))
  (:Pressed
    (if (not (Variables|Default|GetbDisplaying))
      (if (Variables|Default|GetbEnding)
        (CallFunction|JordanEnding)
        (elif (Variables|Default|GetbResolveChoices)
          (Variables|Default|SetbDisplaying true)
          (Widget|RemovefromParent (Variables|Default|GetCurrentDialogueWidget))
          (bind _returnvalue (UserInterface|CreateWidget "/Game/DialogueSystem/Widgets/WI_ChoiceSelection.WI_ChoiceSelection_C" (Game|GetPlayerController 0) self (.responses (Variables|Default|GetCurrentDialogue))))
          (bind _output_get (Variables|Default|SetChoicesWidget _returnvalue))
          (UserInterface|Viewport|AddtoViewport _output_get 0)
          (else
            (CallFunction|DisplayCurrentDialogue)))))))

(event Input|AxisEvents|InputAxisLeftThumbstickX
  (params (AxisValue :type Float%20%28single-precision%29))
  (bind _returnvalue (Game|GetPlayerController 0))
  (bind _returnvalue_2 (Input|AxisValues|GetLeftThumbstickX))
  (bind _returnvalue_3 (Input|AxisValues|GetLeftThumbstickY))
  (bind (_locationx _locationy) (Game|Player|GetMousePosition _returnvalue))
  (Development|PrintString (Utilities|String|ToString(Float) AxisValue) true false "(R=0.000000,G=0.660000,B=1.000000,A=1.000000)" 2.0 "5")
  (if (or (> (Math|Float|Absolute(Float) _returnvalue_2) 0.0) (> (Math|Float|Absolute(Float) _returnvalue_3) 0.0))
    (Class|PlayerController|SetMouseLocation (Game|GetPlayerController 0) (Math|Float|Round (+ _locationx (* _returnvalue_2 (Variables|Default|GetSensiX)))) (Math|Float|Round (+ _locationy (* _returnvalue_3 (Variables|Default|GetSensiY)))))))

(fn ConstructionScript)

(fn SetupScenaro)

(fn ResponseButton
  (params (Affection :type Integer))
  (Variables|Default|SetJordanAffection (+ Affection (Variables|Default|GetJordanAffection)))
  (Utilities|ResolveDialogue)
  (Widget|RemovefromParent (Variables|Default|GetChoicesWidget))
  (Variables|Default|SetbResolveChoices false)
  (CallFunction|DisplayCurrentDialogue))

(fn GetScenarioBackground
  (params (Scenario :type Scenario%20Struct%20Structure))
  (for _array_element (Variables|Default|GetScenarioBackgroundList)
    (if (Utilities|Enum|Equal(Enum) (.scenario _array_element) (.scenario Scenario))
      (return (.texture _array_element))))
  (Development|PrintText "Scenario Background Not Found"))

(fn DisplayCharacter
  (params (SpeakerName :type Text) (Character%20Emotion :type CharacterEmotions%20Enum :default "Normal"))
  (if (Utilities|Enum|Equal(Enum) (Utilities|String|ToString(Text) SpeakerName) (Variables|Default|GetCharacterName))
    (bind _array_element (Utilities|Array|ForEachLoopwithBreak (Variables|Default|GetCharacterDisplayList) :!label _label)
      (:LoopBody
        (if (Utilities|Enum|Equal(Enum) (.characteremotion _array_element) Character%20Emotion)
          (Default|ChangeCharacter (Variables|Default|GetCharacterDisplayWidget) (.charactertexture _array_element))
          (goto _label Break)))
      (:Completed
        (return)))))

(fn GetCharacterDisplayList
  (if (Utilities|Enum|Equal(Enum) (Variables|Default|GetCharacterName) "Jordan")
    (bind _output_get (Variables|Default|SetCharacterDisplayTable "/Game/DialogueSystem/DataTables/Jordan/JordanDisplayTable.JordanDisplayTable"))
    (bind _outrownames (DataTable|GetDataTableRowNames _output_get))
    (for _array_element _outrownames
      (bind _returnvalue (Utilities|GetDataTableRow (Variables|Default|GetCharacterDisplayTable) _array_element)
        (:then
          (Utilities|Array|Add (Variables|Default|GetCharacterDisplayList) _returnvalue))))
    (return)
    (elif (not (Utilities|Enum|Equal(Enum) (Variables|Default|GetCharacterName) "A"))
      (if (Utilities|Enum|Equal(Enum) (Variables|Default|GetCharacterName) "B")
        _))))

(fn SaveGame
  (bind _jordanaffection (Variables|Default|GetJordanAffection))
  (bind _currentscenarioindex (Variables|Default|GetCurrentScenarioIndex))
  (bind _currentdialogueindex (Variables|Default|GetCurrentDialogueIndex))
  (if (Variables|Default|GetbResolveChoices)
    (LocalVariables|SetSaveStruct (Utilities|Struct|MakeSaveStruct 0 _jordanaffection _currentscenarioindex _currentdialogueindex))
    (else
      (LocalVariables|SetSaveStruct (Utilities|Struct|MakeSaveStruct 0 _jordanaffection _currentscenarioindex (- _currentdialogueindex 1)))))
  (bind _returnvalue (SaveGame|CreateSaveGameObject "/Game/DialogueSystem/BP_SaveGame.BP_SaveGame_C"))
  (Variables|/Game/DialogueSystem/BP_SaveGame.BP_SaveGame_C|SetSaveStruct _returnvalue (LocalVariables|GetSaveStruct))
  (SaveGame|SaveGametoSlot _returnvalue "saveslot"))

(fn LoadGame
  (CallFunction|PlayGameMusic)
  (bind _returnvalue (SaveGame|LoadGamefromSlot "saveslot"))
  (bind _asbp_save_game (Utilities|Casting|CastToBP_SaveGame _returnvalue))
  (Variables|Default|SetJordanAffection (.affection (Variables|/Game/DialogueSystem/BP_SaveGame.BP_SaveGame_C|GetSaveStruct _asbp_save_game)))
  (Variables|Default|SetCurrentScenarioIndex (.scenarioid (Variables|/Game/DialogueSystem/BP_SaveGame.BP_SaveGame_C|GetSaveStruct _asbp_save_game)))
  (Variables|Default|SetCurrentDialogueIndex (.dialogueid (Variables|/Game/DialogueSystem/BP_SaveGame.BP_SaveGame_C|GetSaveStruct _asbp_save_game)))
  (Variables|Default|SetbDisplaying false)
  (Variables|Default|SetbScenarioChange true)
  (Variables|Default|SetbResolveChoices false)
  (Variables|Default|SetCurrentScenario (Utilities|Array|Get(acopy) (Variables|Default|GetJordanScenarios) (Variables|Default|GetCurrentScenarioIndex)))
  (CallFunction|DisplayCurrentDialogue))

(fn StartButtonFunc
  (params (CharacterName :type String))
  (Widget|RemovefromParent (Variables|Default|GetMainMenuWidget))
  (CallFunction|StartGame))

(fn LoadGameButton
  (Widget|RemovefromParent (Variables|Default|GetMainMenuWidget))
  (Utilities|GameInit)
  (bind _returnvalue (UserInterface|CreateWidget "/Game/DialogueSystem/Widgets/WI_Dialogue.WI_Dialogue_C" 0 "Init" "" 0))
  (Variables|Default|SetCurrentDialogueWidget _returnvalue)
  (CallFunction|LoadGame))

(fn PlayGameMusic
  (bind _mainmenumusic (Variables|Default|GetMainMenuMusic))
  (Utilities|IsValid _mainmenumusic
    (:Is%20Valid
      (if (Audio|Components|Audio|IsPlaying _mainmenumusic)
        (Audio|Components|Audio|Stop _mainmenumusic)))
    (:Is%20Not%20Valid
      _))
  (if (Audio|Components|Audio|IsPlaying (Variables|Default|GetGameplayMusic))
    _
    (else
      (Audio|Components|Audio|Play (Variables|Default|GetGameplayMusic) 0.0)))
  (return))